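; Playable tobiko sushi character that knocks other sushi characters away on collision and shows a player name tag.
; Capsule hits play a crash sound and launch salmon, tuna or tobiko characters at twice this character's velocity, cached each tick; salmon also requires a camera-forward sphere trace hit.
; After a delay, the local player's name passes through server and multicast events into PlayerName, whose RepNotify retries until the widget is valid.
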(event OnComponentHit(CapsuleComponent)
  (params (HitComponent :type Primitive%20Component%20Object%20Reference) (OtherActor :type Actor%20Object%20Reference) (OtherComp :type Primitive%20Component%20Object%20Reference) (NormalImpulse :type Vector :default "0, 0, 0") (Hit :type Hit%20Result%20Structure%20%28by%20ref%29))
  (bind _followcamera (Variables|Default|GetFollowCamera))
  (bind _returnvalue (Transformation|GetWorldLocation _followcamera))
  (Audio|PlaySound2D "/Game/Sounds/_sushicrash_270554__littlerobotsoundfactory__warpdrive_02-_AudioTrimmer_com_._sushicrash_270554__littlerobotsoundfactory__warpdrive_02-_AudioTrimmer_com_" 1.0 1.0 0.0 0 0)
  (Utilities|FlowControl|Sequence
    (:then_0
      (bind _assalmon_sushi_char (Utilities|Casting|CastTosalmonSushi_Char OtherActor))
      (bind (_outhit _returnvalue_2) (Collision|SphereTraceForObjects _returnvalue (+ _returnvalue (* (Math|Vector|GetForwardVector (Transformation|GetWorldRotation _followcamera)) "1000.000000,1000.000000,1000.000000")) 1e+01 (Utilities|Array|MakeArray "ObjectTypeQuery3") false 0 "None"))
      (if _returnvalue_2
        (Character|LaunchCharacter _assalmon_sushi_char (Variables|Default|GetForward) false false)))
    (:then_1
      (bind _astuna_sushi_char (Utilities|Casting|CastTotunaSushi_Char OtherActor))
      (Character|LaunchCharacter _astuna_sushi_char (Variables|Default|GetForward) false false))
    (:then_2
      (bind _astobiko_sushi_char (Utilities|Casting|CastTotobikoSushi_Char OtherActor))
      (Character|LaunchCharacter _astobiko_sushi_char (Variables|Default|GetForward) false false))))

(event EventBeginPlay
  (Utilities|FlowControl|Delay 1.0)
  (CallFunction|SetUpLocal))

(event EventTick
  (params (DeltaSeconds :type Float%20%28single-precision%29))
  (Variables|Default|SetForward (* (Transformation|GetVelocity) "2.000000,2.000000,2.000000")))

(fn ConstructionScript)

(fn SetUpLocal
  (if (Pawn|IsLocallyControlled)
    (CallFunction|SetNameTagServer (Utilities|Text|ToText(String) (PlayerState|GetPlayerName (Variables|/Script/Engine.Controller|GetPlayerState (Game|GetPlayerController 0)))))))

(fn OnRepPlayerName
  (bind _nametag (Variables|Default|GetNameTag))
  (bind _returnvalue (UserInterface|GetWidget _nametag))
  (Utilities|IsValid _returnvalue
    (:Is%20Valid
      (bind _asbp_name_tag (Utilities|Casting|CastToBP_NameTag _returnvalue))
      (Default|SetText _asbp_name_tag (Variables|Default|GetPlayerName))
      (Development|SetHiddeninGame (Variables|Default|GetNameTag) false false))
    (:Is%20Not%20Valid
      (Utilities|Time|SetTimerbyFunctionName 0 "OnRep_PlayerName" 0.1))))

(event Custom|SetNameTagServer
  (params (PlayerName :type Text))
  (CallFunction|SetNameTagMulticast PlayerName))

(event Custom|SetNameTagMulticast
  (params (PlayerName :type Text))
  (Variables|Default|SetPlayerName PlayerName))