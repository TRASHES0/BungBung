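; MyBungBungCharacter is a character Blueprint that knocks other characters of the same class away on collision.
; Tick stores twice the character's current velocity as a launch vector.
; On a capsule hit with another such character, a sphere trace runs forward from the follow camera against Pawns, with persistent debug drawing.
; Any trace hit launches the collided character with the stored velocity, regardless of which Pawn the trace found.
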(event OnComponentHit(CapsuleComponent)
  (params (HitComponent :type Primitive%20Component%20Object%20Reference) (OtherActor :type Actor%20Object%20Reference) (OtherComp :type Primitive%20Component%20Object%20Reference) (NormalImpulse :type Vector :default "0, 0, 0") (Hit :type Hit%20Result%20Structure%20%28by%20ref%29))
  (bind _followcamera (Variables|Default|GetFollowCamera))
  (bind _returnvalue (Transformation|GetWorldLocation _followcamera))
  (bind _asmy_bung_bung_character (Utilities|Casting|CastToMyBungBungCharacter OtherActor))
  (bind (_outhit _returnvalue_2) (Collision|SphereTraceForObjects _returnvalue (+ _returnvalue (* (Math|Vector|GetForwardVector (Transformation|GetWorldRotation _followcamera)) "1000.000000,1000.000000,1000.000000")) 1e+01 (Utilities|Array|MakeArray "ObjectTypeQuery3") false 0 "Persistent"))
  (if _returnvalue_2
    (Character|LaunchCharacter _asmy_bung_bung_character (Variables|Default|GetForward) false false)))

(event EventBeginPlay)

(event Collision|EventActorBeginOverlap
  (params (OtherActor :type Actor%20Object%20Reference)))

(event EventTick
  (params (DeltaSeconds :type Float%20%28single-precision%29))
  (Variables|Default|SetForward (* (Transformation|GetVelocity) "2.000000,2.000000,2.000000")))

(fn ConstructionScript)