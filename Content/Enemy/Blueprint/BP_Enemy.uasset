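; Enemy character that follows sensed Player-tagged actors and bumps sushi characters or other enemies on contact.
; AI perception writes the target to the blackboard, and a short timer clears it after sight or sensing is lost.
; Capsule hits launch characters using velocity cached each Tick.
; Only the salmon branch recoils the enemy itself; other branches apply both forward and reverse launches to the hit character.
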(event OnTargetPerceptionUpdated(AIPerception)
  (params (Actor :type Actor%20Object%20Reference) (Stimulus :type AI%20Stimulus%20Structure))
  (Utilities|ProcessTilmuli Actor Stimulus
    (:FollowNewActor
      (CallFunction|FollowActorTarget Actor))
    (:LostTrackOfTarget
      (CallFunction|LostTrackOfTarget))))

(event OnComponentHit(CapsuleComponent)
  (params (HitComponent :type Primitive%20Component%20Object%20Reference) (OtherActor :type Actor%20Object%20Reference) (OtherComp :type Primitive%20Component%20Object%20Reference) (NormalImpulse :type Vector :default "0, 0, 0") (Hit :type Hit%20Result%20Structure%20%28by%20ref%29))
  (bind _speed (Variables|Default|GetSpeed))
  (bind _speed_2 (Variables|Default|GetSpeed))
  (bind _speed_3 (Variables|Default|GetSpeed))
  (bind _speed_4 (Variables|Default|GetSpeed))
  (Utilities|FlowControl|Sequence
    (:then_0
      (bind _assalmon_sushi_char (Utilities|Casting|CastTosalmonSushi_Char OtherActor))
      (Character|LaunchCharacter _assalmon_sushi_char _speed_2 false false)
      (Character|LaunchCharacter (* _speed_2 "-1.500000,-1.500000,-1.500000") false false))
    (:then_1
      (bind _astuna_sushi_char (Utilities|Casting|CastTotunaSushi_Char OtherActor))
      (Character|LaunchCharacter _astuna_sushi_char _speed_3 false false)
      (Character|LaunchCharacter _astuna_sushi_char (* _speed_3 "-1.500000,-1.500000,-1.500000") false false))
    (:then_2
      (bind _astobiko_sushi_char (Utilities|Casting|CastTotobikoSushi_Char OtherActor))
      (Character|LaunchCharacter _astobiko_sushi_char _speed_4 false false)
      (Character|LaunchCharacter _astobiko_sushi_char (* _speed_4 "-1.500000,-1.500000,-1.500000") false false))
    (:then_3
      (bind _asbp_enemy (Utilities|Casting|CastToBP_Enemy OtherActor))
      (Character|LaunchCharacter _asbp_enemy _speed false false)
      (Character|LaunchCharacter _asbp_enemy (* _speed "-1.500000,-1.500000,-1.500000") false false))))

(event EventBeginPlay)

(event Collision|EventActorBeginOverlap
  (params (OtherActor :type Actor%20Object%20Reference)))

(event EventTick
  (params (DeltaSeconds :type Float%20%28single-precision%29))
  (Variables|Default|SetSpeed (Transformation|GetVelocity)))

(fn ConstructionScript)

(fn FollowActorTarget
  (params (ObjectValue :type Object%20Object%20Reference))
  (AI|Components|Blackboard|SetValueasObject (AI|GetBlackboard 0) (Variables|Default|GetFollowTargetKey) ObjectValue)
  (return))

(fn LostTrackOfTarget
  (bind _returnvalue (Utilities|Time|SetTimerbyFunctionName 0 "ForgotAboutTarget" 1.0))
  (Variables|Default|SetDurationTimer _returnvalue)
  (return))

(fn ForgotAboutTarget
  (AI|Components|Blackboard|SetValueasObject (AI|GetBlackboard 0) (Variables|Default|GetFollowTargetKey) 0)
  (return))