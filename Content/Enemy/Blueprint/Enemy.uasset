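; Enemy AI Blueprint with helpers for following a sensed actor and forgetting it after losing track.
; The ProcessTilmuli macro checks the actor's tags and sensing success, then routes to follow, lost-track or ignore outputs.
; Follow writes the actor to the blackboard's follow-target key, while losing track starts a memory-duration timer that later clears it.
; No event wiring connects the macro to these functions here.
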(fn ConstructionScript)

(fn FollowActorTarget
  (params (ObjectValue :type Object%20Object%20Reference))
  (AI|Components|Blackboard|SetValueasObject (AI|GetBlackboard 0) (Variables|Default|GetFollowTargetKey) ObjectValue)
  (return))

(fn LostTrackOfTarget
  (bind _returnvalue (Utilities|Time|SetTimerbyFunctionName 0 "ForgotAboutTarget" (Variables|Default|GetMemoryDuration)))
  (Variables|Default|SetDurationTimer _returnvalue)
  (return))

(fn ForgotAboutTarget
  (AI|Components|Blackboard|SetValueasObject (AI|GetBlackboard 0) (Variables|Default|GetFollowTargetKey) 0)
  (return))